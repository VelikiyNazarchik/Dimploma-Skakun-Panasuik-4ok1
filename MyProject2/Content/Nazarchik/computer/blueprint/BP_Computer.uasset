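; Interactive computer actor that shows a terminal screen on a 3D widget component in the world.
; TurnOn calls TurnOnTerminal, which creates a Terminalko_WB widget, assigns it to the component, enables input and shows the mouse cursor.
; TurnOffTerminal, not called in this Blueprint, destroys the widget component itself and hides the cursor.
; The box overlap event is empty, and leftover unwired nodes include an older viewport-based Terminal_WB version.
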(event `Turn On`
  (`self.Turn_On_Terminal`))

(event `self.Box.OnComponentBeginOverlap`
  (params (OverlappedComponent :type "PrimitiveComponent Object Reference") (OtherActor :type "Actor Object Reference") (OtherComp :type "PrimitiveComponent Object Reference") (OtherBodyIndex :type Integer) (bFromSweep :type Boolean) (SweepResult :type "HitResult Structure (by ref)")))

(event `Key|E`
  (params (Key :type "Key Structure")))

(fn `Turn_Off_Terminal`
  (bind _ascharacter (cast `Character` (`GameplayStatics.GetPlayerPawn` 0)))
  (bind _returnvalue (`Pawn.GetLocalViewingPlayerController` _ascharacter))
  (set `self.PlayerControl` _returnvalue)
  (`ActorComponent.K2_DestroyComponent` (`self.Widget`))
  (set `PlayerController.bShowMouseCursor` false _returnvalue))

(fn `Turn_On_Terminal`
  (bind _widget (`self.Widget`))
  (bind _ascharacter (cast `Character` (`GameplayStatics.GetPlayerPawn` 0)))
  (bind _output_get (set `self.PlayerControl` (`Pawn.GetLocalViewingPlayerController` _ascharacter)))
  (bind _returnvalue (`|GenericCreateObject` _widget "/Game/Nazarchik/computer/Widget/Terminalko_WB.Terminalko_WB_C"))
  (`PrimitiveComponent.SetBoundsScale` _widget 0.1)
  (bind _output_get_2 (set `self.3DnewWidget` _returnvalue))
  (`WidgetComponent.SetWidget` _widget _output_get_2)
  (`self.EnableInput` _output_get)
  (set `PlayerController.bShowMouseCursor` true _output_get))

(fn `UserConstructionScript`)