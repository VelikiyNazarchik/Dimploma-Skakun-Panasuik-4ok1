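; Shardwretch enemy character Blueprint, providing the attack, patrol and movement hooks for this creature.
; The attack event plays the Shardwretch attack montage and calls OnAttackEnd whether it completes or is interrupted.
; Getter functions return fixed attack and defend radii and the assigned patrol route, while SetMoveSpeed maps a movement state from idle to running onto the walk speed cap.
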(event `attack`
  (`|PlayMontage` (`self.Mesh`) "/Game/Nazarchik/enemies/Shardwretch/Animations/attackShardwretch_AnimM.attackShardwretch_AnimM"
    (:`OnCompleted`
      _)
    (:`OnInterrupted`
      _))
  (`self.OnAttackEnd`))

(fn `GetIdealRange`
  (returns (AttackRadius :type "Float (double-precision)") (DefendRadius :type "Float (double-precision)"))
  (return 150.0 350.0))

(fn `GetPatrolRoute`
  (returns (PatrolRoute :type "/Game/Nazarchik/enemies/Shardwretch/Behaviour/Shardwretch_PatrolRoute_BP Object Reference"))
  (return (`self.PatrolRoute`)))

(fn `SetMoveSpeed`
  (params (Speed :type "/Game/Nazarchik/enemies/Shardwretch/Behaviour/Enums/Shardwretch_MoveSpeed_E Enum" :default "NewEnumerator0"))
  (returns (SpeedValue :type "Float (double-precision)"))
  (bind _output_get (set `CharacterMovementComponent.MaxWalkSpeed` (select `/Game/Nazarchik/enemies/Shardwretch/Behaviour/Enums/Shardwretch_MoveSpeed_E` Speed :`NewEnumerator1` 100.0 :`NewEnumerator4` 150.0 :`NewEnumerator2` 400.0 :!type "Float (single-precision)") (`self.CharacterMovement`)))
  (return _output_get))

(fn `UserConstructionScript`)