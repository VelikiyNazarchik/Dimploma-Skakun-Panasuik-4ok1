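; Pudge enemy character that carries a hook weapon and supplies combat ranges, patrol route and walk speeds, likely for AI control.
; On BeginPlay it spawns an enlarged crystal and randomly attaches it to a neck, forearm or hand socket; one roll leaves it unattached.
; Attacks play a montage and signal their end on completion or interruption.
; Wielding spawns the hook on the weapon socket; sheathing signals and destroys it.
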(event `Key|J`
  (params (Key :type "Key Structure")))

(event `self.ReceiveBeginPlay`
  (bind _returnvalue (`|SpawnActorFromClass` "/Game/Nazarchik/Crystal_generation.Crystal_generation_C" (`KismetMathLibrary.MakeTransform` (0.0 0.0 0.0) (struct) (5.0 5.0 5.0)) "Undefined" "MultiplyWithRoot" null null))
  (switch `int` (`KismetMathLibrary.RandomIntegerInRange` 0 3)
    (:`0`
      (set `self.socket` "NeckSocket"))
    (:`1`
      (set `self.socket` "RightForeArmSocket"))
    (:`2`
      (set `self.socket` "RightHandIndex1Socket")))
  (`self.K2_AttachToComponent` _returnvalue (`self.Mesh`) (`self.socket`) "SnapToTarget" "SnapToTarget" "KeepRelative" false)
  (`KismetSystemLibrary.PrintString` "DOWN"))

(event `attack`
  (`|PlayMontage` (`self.Mesh`) "/Game/Nazarchik/enemy/animations/Attacking_AM.Attacking_AM"
    (:`OnCompleted`
      _)
    (:`OnInterrupted`
      _))
  (`self.OnAttackEnd`))

(event `WeildWeapon`
  (bind _returnvalue (`|SpawnActorFromClass` "/Game/Nazarchik/enemy/weapon/1/hoock_BP.hoock_BP_C" (`self.GetTransform`) "Undefined" "MultiplyWithRoot" null null))
  (bind _output_get (set `self.Weapon` _returnvalue))
  (`self.K2_AttachToComponent` _output_get (`self.Mesh`) "weapon_r" "SnapToTarget" "SnapToTarget" "SnapToTarget" true)
  (set `self.IsWeildingWeapon` true))

(event `SheathWeapon`
  (set `self.IsWeildingWeapon` false)
  (`self.OnSheathWeapon`)
  (`self.K2_DestroyActor` (`self.Weapon`)))

(fn `GetIdealRange`
  (returns (AttackRadius :type "Float (double-precision)") (DefendRadius :type "Float (double-precision)"))
  (return 150.0 350.0))

(fn `GetPatrolRoute`
  (returns (PatrolRoute :type "/Game/Nazarchik/enemy/Beheviour/PatrolRoute_BP Object Reference"))
  (return (`self.PatrolRoute`)))

(fn `SetMoveSpeed`
  (params (Speed :type "/Game/Nazarchik/enemy/Beheviour/Enums/MoveSpeed_E Enum" :default "NewEnumerator0"))
  (returns (SpeedValue :type "Float (double-precision)"))
  (bind _output_get (set `CharacterMovementComponent.MaxWalkSpeed` (select `/Game/Nazarchik/enemy/Beheviour/Enums/MoveSpeed_E` Speed :`NewEnumerator1` 100.0 :`NewEnumerator2` 600.0 :!type "Float (single-precision)") (`self.CharacterMovement`)))
  (return _output_get))

(fn `UserConstructionScript`)