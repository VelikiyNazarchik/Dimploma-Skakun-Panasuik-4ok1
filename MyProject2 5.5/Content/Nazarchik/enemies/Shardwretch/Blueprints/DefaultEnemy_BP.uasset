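; Base Shardwretch enemy character that holds health and exposes combat range, patrol route and movement speed through getters and a setter.
; AnyDamage subtracts from clamped Health and flags IsDead with a debug print at zero, while Heal restores a fraction of MaxHealth.
; SetMoveSpeed maps a movement state to the CharacterMovement walk speed, and GetIdealRange returns fixed attack and defend radii.
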(event `self.ReceiveAnyDamage`
  (params (Damage :type "Float (single-precision)") (DamageType :type "DamageType Object Reference") (InstigatedBy :type "Controller Object Reference") (DamageCauser :type "Actor Object Reference"))
  (bind _output_get (set `self.Health` (`KismetMathLibrary.FClamp` (- (`self.Health`) Damage) 0.0 (`self.MaxHealth`))))
  (if (<= _output_get 0.0)
    (set `self.IsDead` true)
    (`KismetSystemLibrary.PrintString` "Dead")))

(event `/Game/Nazarchik/enemies/Shardwretch/Behaviour/Base_EnemyAI_BPI.Heal`
  (params (`Heal Precentage` :type "Float (double-precision)"))
  (set `self.Health` (`KismetMathLibrary.FClamp` (+ (`self.Health`) (* `Heal Precentage` (`self.MaxHealth`))) 0.0 (`self.MaxHealth`))))

(fn `GetCurrentHealth`
  (returns (Health :type "Float (double-precision)"))
  (return (`self.Health`)))

(fn `GetIdealRange`
  (returns (AttackRadius :type "Float (double-precision)") (DefendRadius :type "Float (double-precision)"))
  (return 150.0 350.0))

(fn `GetMaxHealth`
  (returns (MaxHealth :type "Float (double-precision)"))
  (return (`self.MaxHealth`)))

(fn `GetPatrolRoute`
  (returns (PatrolRoute :type "/Game/Nazarchik/enemies/Shardwretch/Behaviour/Shardwretch_PatrolRoute_BP Object Reference"))
  (return (`self.PatrolRoute`)))

(fn `SetMoveSpeed`
  (params (Speed :type "/Game/Nazarchik/enemies/Shardwretch/Behaviour/Enums/MoveSpeed_E Enum" :default "NewEnumerator0"))
  (returns (SpeedValue :type "Float (double-precision)"))
  (bind _output_get (set `CharacterMovementComponent.MaxWalkSpeed` (select `/Game/Nazarchik/enemies/Shardwretch/Behaviour/Enums/MoveSpeed_E` Speed :`NewEnumerator1` 100.0 :`NewEnumerator4` 150.0 :`NewEnumerator2` 400.0 :!type "Float (single-precision)") (`self.CharacterMovement`)))
  (return _output_get))

(fn `UserConstructionScript`)