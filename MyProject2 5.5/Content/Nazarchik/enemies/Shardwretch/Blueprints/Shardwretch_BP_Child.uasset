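; Shardwretch enemy variant, a Blueprint child that makes a short-range melee attack and starts with 200 health in its damage component.
; Attack plays a sped-up montage, whose notify sphere-traces forward for pawns and sends damage through a damage message.
; Montage completion or interruption signals attack end.
; It supplies a close attack range, always reports alive and returns zero from Heal; the parent construction script is not called.
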(event `/Game/Nazarchik/enemies/Shardwretch/Behaviour/Base_EnemyAI_BPI.Attack`
  (bind _returnvalue (`self.K2_GetActorLocation`))
  (bind _notifyname (`|PlayMontage` (`self.Mesh`) "/Game/Nazarchik/enemies/Shardwretch/Animations/NEW/Shardwretch_New_Attack_1.Shardwretch_New_Attack_1" 2.0)
    (:`OnCompleted`
      (`self.OnAttackEnd` :!label _label))
    (:`OnInterrupted`
      (goto _label))
    (:`OnNotifyBegin`
      (switch `name` _notifyname
        (:`Hit`
          (bind (_outhit _returnvalue_2) (`KismetSystemLibrary.SphereTraceSingleForObjects` :`Start` _returnvalue :`End` (+ _returnvalue (* 200.0 (`self.GetActorForwardVector`))) :`Radius` 20.0 :`ObjectTypes` (`|MakeArray` "ObjectTypeQuery3" :!type "EObjectTypeQuery Enum") :`DrawDebugType` "ForDuration"))
          (if _returnvalue_2
            (message `/Game/Nazarchik/enemies/Damage_system/Damageble_BPI.TakeDamage` (`.HitActor` (`GameplayStatics.BreakHitResult` _outhit)) (make `/Game/Nazarchik/enemies/Damage_system/DamageInfo_S` 5.0 "NewEnumerator1"))))))))

(fn `GetIdealRange`
  (returns (AttackRadius :type "Float (double-precision)") (DefendRadius :type "Float (double-precision)"))
  (return 75.0 0.0))

(fn `Heal`
  (params (Amount :type "Float (double-precision)"))
  (returns (NewHealth :type "Float (double-precision)"))
  (return 0.0))

(fn `IsDead`
  (returns (IsDead :type Boolean))
  (return false))

(fn `UserConstructionScript`
  (bind _damagesystem_bpc (`self.DamageSystem_BPC`))
  (set `/Game/Nazarchik/enemies/Damage_system/DamageSystem_BPC.MaxHealth` 200.0 _damagesystem_bpc)
  (set `/Game/Nazarchik/enemies/Damage_system/DamageSystem_BPC.Health` 200.0 _damagesystem_bpc))