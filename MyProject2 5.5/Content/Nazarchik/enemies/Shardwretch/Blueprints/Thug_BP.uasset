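; Thug enemy Blueprint that attacks with a pistol and supplies its movement speeds and ideal combat ranges.
; Attack plays a shot montage; on completion or interruption it plays a placeholder ping and traces from the pistol to the AI controller's target.
; An unblocked trace applies damage, then attack end fires if the target was valid.
; Debug trace drawing and health printing remain, and IsDead always returns false.
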(event `self.ReceiveBeginPlay`
  (`parent.ReceiveBeginPlay`))

(event `/Game/Nazarchik/enemies/Shardwretch/Behaviour/Base_EnemyAI_BPI.Attack`
  (bind _returnvalue (`SceneComponent.GetSocketLocation` (`self.Pistol`) "None"))
  (`|PlayMontage` (`self.Mesh`) "/Game/Nazarchik/enemies/Thug/Animations/Thug_shot_AnimM.Thug_shot_AnimM"
    (:`OnCompleted`
      _)
    (:`OnInterrupted`
      _))
  (`GameplayStatics.PlaySoundAtLocation` "/Engine/EngineSounds/1kSineTonePing.1kSineTonePing" _returnvalue (struct) 1.0 1.0 0.0 null null null null)
  (bind _asenemy_base_aic (cast `/Game/Nazarchik/enemies/Shardwretch/Behaviour/EnemyBase_AIC` (`AIBlueprintHelperLibrary.GetAIController` self)))
  (bind _attack_target (`/Game/Nazarchik/enemies/Shardwretch/Behaviour/EnemyBase_AIC.Attack Target` _asenemy_base_aic)
    (:`then`
      (bind (_outhit _returnvalue_2) (`KismetSystemLibrary.LineTraceSingle` :`Start` _returnvalue :`End` (`self.K2_GetActorLocation` _attack_target) :`TraceChannel` "TraceTypeQuery1" :`DrawDebugType` "ForDuration"))
      (if (not _returnvalue_2)
        (message `/Game/Nazarchik/enemies/Damage_system/Damageble_BPI.TakeDamage` _attack_target (make `/Game/Nazarchik/enemies/Damage_system/DamageInfo_S` 25.0 "NewEnumerator2")))
      (`self.OnAttackEnd`)
      (bind _returnvalue_3 (`GameplayStatics.GetActorOfClass` "/Game/Sonik/New_Character/Character.Character_C"))
      (bind _health (`/Game/Nazarchik/enemies/Damage_system/Damageble_BPI.GetCurrentHealth` _returnvalue_3))
      (`KismetSystemLibrary.PrintString` (`KismetStringLibrary.Conv_DoubleToString` _health)))
    (:`else`)))

(fn `GetIdealRange`
  (returns (AttackRadius :type "Float (double-precision)") (DefendRadius :type "Float (double-precision)"))
  (return 800.0 600.0))

(fn `IsDead`
  (returns (IsDead :type Boolean))
  (return false))

(fn `SetMoveSpeed`
  (params (Speed :type "/Game/Nazarchik/enemies/Shardwretch/Behaviour/Enums/MoveSpeed_E Enum" :default "NewEnumerator0"))
  (returns (SpeedValue :type "Float (double-precision)"))
  (bind _output_get (set `CharacterMovementComponent.MaxWalkSpeed` (select `/Game/Nazarchik/enemies/Shardwretch/Behaviour/Enums/MoveSpeed_E` Speed :`NewEnumerator1` 200.0 :`NewEnumerator4` 150.0 :`NewEnumerator2` 600.0 :!type "Float (single-precision)") (`self.CharacterMovement`)))
  (return _output_get))

(fn `UserConstructionScript`
  (`parent.UserConstructionScript`))