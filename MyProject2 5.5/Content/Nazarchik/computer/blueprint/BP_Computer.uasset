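; BP_Computer is an in-world computer actor that gives a first-person character access to a terminal screen when they come near.
; Box overlap by a Character_FPS builds a Terminalko_WB, assigns it to the Widget component, enables the character's input and shows the mouse cursor.
; Ending the overlap hides the cursor again, without checking which actor left.
; An older viewport-based Terminal_WB path remains in the graph but never runs.
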(event `self.Box.OnComponentBeginOverlap`
  (params (OverlappedComponent :type "PrimitiveComponent Object Reference") (OtherActor :type "Actor Object Reference") (OtherComp :type "PrimitiveComponent Object Reference") (OtherBodyIndex :type Integer) (bFromSweep :type Boolean) (SweepResult :type "HitResult Structure (by ref)"))
  (bind _widget (`self.Widget`))
  (bind _ascharacter_fps (cast `/Game/Nazarchik/Character/Blueprints/Character_FPS` OtherActor))
  (set `self.PlayerControl` (`Pawn.GetLocalViewingPlayerController` _ascharacter_fps))
  (bind _returnvalue (`|GenericCreateObject` _widget "/Game/Nazarchik/computer/Widget/Terminalko_WB.Terminalko_WB_C"))
  (`PrimitiveComponent.SetBoundsScale` _widget 0.1)
  (bind _output_get (set `self.3DnewWidget` _returnvalue))
  (`WidgetComponent.SetWidget` _widget _output_get)
  (`self.EnableInput` _ascharacter_fps (`self.PlayerControl`))
  (set `PlayerController.bShowMouseCursor` true (`self.PlayerControl`)))

(event `self.Box.OnComponentEndOverlap`
  (params (OverlappedComponent :type "PrimitiveComponent Object Reference") (OtherActor :type "Actor Object Reference") (OtherComp :type "PrimitiveComponent Object Reference") (OtherBodyIndex :type Integer))
  (set `PlayerController.bShowMouseCursor` false (`self.PlayerControl`)))

(event `Key|E`
  (params (Key :type "Key Structure")))

(fn `UserConstructionScript`)