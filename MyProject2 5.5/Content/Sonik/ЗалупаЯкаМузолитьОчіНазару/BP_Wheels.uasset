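; BP_Wheels is a wheel item that the player can interact with to attach it to their character.
; On BeginPlay it sets its static mesh from the WheelsDataTable row selected by RowName.
; Interact snaps it to a socket on player 0's character mesh, keeping world scale, and returns true.
; AttachToCar is a stub returning false, NewFunction0 is empty, and both physics toggles are unwired.
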(event `self.ReceiveBeginPlay`
  (bind _returnvalue (`|GetDataTableRow` "/Game/Sonik/ЗалупаЯкаМузолитьОчіНазару/WheelsDataTable.WheelsDataTable" (`self.Row Name`))
    (:`then`
      (`StaticMeshComponent.SetStaticMesh` (`self.StaticMesh`) (`.Mesh_4_A02FEE254184BC756B3C92B31806957D` (break `/Game/Sonik/ЗалупаЯкаМузолитьОчіНазару/WheelsStruct` _returnvalue))))))

(fn `Attach to car`
  (params (NewParam1 :type Boolean) (zal :type "Actor Object Reference") (NewParam3 :type "Actor Object Reference"))
  (returns (NewParam :type Boolean) (NewParam4 :type "Actor Object Reference"))
  (return false null))

(fn `Interact`
  (params (NewParam :type Boolean) (NewParam1 :type "ActorComponent Object Reference") (`Ahuet da?` :type "Actor Object Reference"))
  (returns (Interacted :type Boolean))
  (`self.K2_AttachToComponent` (`Character.Mesh` (`GameplayStatics.GetPlayerCharacter` 0)) "УEBU" "SnapToTarget" "SnapToTarget" "KeepWorld")
  (return true))

(fn `NewFunction_0`
  (params (NewParam :type "Actor Object Reference"))
  (returns (NewParam1 :type "Actor Object Reference"))
  (return null))

(fn `UserConstructionScript`)