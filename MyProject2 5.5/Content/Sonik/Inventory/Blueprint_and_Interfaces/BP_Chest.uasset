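; BP_Chest is an interactable storage chest with outline highlighting that opens the inventory UI in its Chest position.
; On BeginPlay it spawns a hidden, non-simulating BackPack_Master far below the world as its 30-slot container.
; Buy and sell events remove and add items in that backpack, whose slots also serve item checks and retrieval.
; HasSpace fails only when no slot is empty and the item's data row is missing.
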(event `self.ReceiveBeginPlay`
  (bind _equipbackpack (`self.EquipBackpack`))
  (bind _returnvalue (`|SpawnActorFromClass` :`Class` "/Game/Sonik/Inventory/Blueprint_and_Interfaces/BackPack_Master.BackPack_Master_C" :`SpawnTransform` (`KismetMathLibrary.MakeTransform` (0.0 0.0 -10000.0)) :`CollisionHandlingOverride` "Undefined" :`TransformScaleMethod` "MultiplyWithRoot" :`Instigator` null))
  (bind _output_get (set `self.EquipBackpack` _returnvalue))
  (`KismetArrayLibrary.Array_Resize` (`/Game/Sonik/Inventory/Blueprint_and_Interfaces/BackPack_Master.PlayerSlots` _output_get) 30)
  (`self.SetActorHiddenInGame` _equipbackpack true)
  (`PrimitiveComponent.SetSimulatePhysics` (`StaticMeshActor.StaticMeshComponent` _equipbackpack) false))

(event `/Game/Sonik/Inventory/Blueprint_and_Interfaces/OutlineInterface.OutlineInteraction`
  (params (ON :type Boolean))
  (bind _staticmeshcomponent (`self.StaticMeshComponent`))
  (if ON
    (`PrimitiveComponent.SetRenderCustomDepth` _staticmeshcomponent true)
    (`PrimitiveComponent.SetCustomDepthStencilValue` _staticmeshcomponent 2)
    (else
      (`PrimitiveComponent.SetRenderCustomDepth` _staticmeshcomponent false)
      (`PrimitiveComponent.SetCustomDepthStencilValue` _staticmeshcomponent 0))))

(event `/Game/Sonik/Inventory/Blueprint_and_Interfaces/AI_Interaction.StartInteraction`
  (params (Player :type "/Game/Sonik/New_Character/Character Object Reference"))
  (set `/Game/Sonik/New_Character/Character.Interactebl` self Player)
  (`/Game/Sonik/New_Character/Character.CreateWidget` Player "/Game/Sonik/Inventory/UI/UI_Inventory.UI_Inventory_C" "Chest"))

(event `/Game/Sonik/Inventory/Blueprint_and_Interfaces/AI_Interaction.SellItem`
  (params (Item :type "/Game/Sonik/Inventory/Structure/S_Slots Structure"))
  (`/Game/Sonik/Inventory/Blueprint_and_Interfaces/BackPack_Master.AddItem` (`self.EquipBackpack`) Item))

(event `/Game/Sonik/Inventory/Blueprint_and_Interfaces/AI_Interaction.BuyItem`
  (params (Index :type Integer) (Item :type "/Game/Sonik/Inventory/Structure/S_Slots Structure"))
  (`/Game/Sonik/Inventory/Blueprint_and_Interfaces/BackPack_Master.RemoveAmountAtIndex` (`self.EquipBackpack`) Index Item_Amount_5_190B8E8A4A3751A596D8F1A8DA065465))

(fn `HasSpace`
  (params (Item :type "/Game/Sonik/Inventory/Structure/S_Slots Structure"))
  (returns (Returne :type Boolean))
  (bind (_datatable _rowname) (break `DataTableRowHandle` (`.Item_4_27233E2C43F0E942A1D6938F2A227CD8` (break `/Game/Sonik/Inventory/Structure/S_Slots` Item))))
  (bind _succes (`/Game/Sonik/Inventory/Blueprint_and_Interfaces/BackPack_Master.FindEmptySlot` (`self.EquipBackpack`)))
  (if _succes
    (return true)
    (else
      (bind _returnvalue (`|GetDataTableRow` _datatable _rowname)
        (:`then`
          (if (`.CanStack_13_EE9C68654E665B3DD19AFEB7618792C9` (break `/Game/Sonik/Inventory/Structure/S_Inventory` _returnvalue))
            (bind _succes_2 (`/Game/Sonik/Inventory/Blueprint_and_Interfaces/BackPack_Master.FindStack` (`self.EquipBackpack`) Item))
            (if _succes_2
              (return true)
              (else
                (return true)))
            (else
              (return true))))
        (:`RowNotFound`
          (return false))))))

(fn `IsItemAvaible`
  (params (Item :type "/Game/Sonik/Inventory/Structure/S_Slots Structure") (Index :type Integer))
  (returns (Returne :type Boolean))
  (return (== (`.RowName` (break `DataTableRowHandle` (`.Item_4_27233E2C43F0E942A1D6938F2A227CD8` (break `/Game/Sonik/Inventory/Structure/S_Slots` Item)))) (`.RowName` (break `DataTableRowHandle` (break `/Game/Sonik/Inventory/Structure/S_Slots` (`|GetArrayItem` (`/Game/Sonik/Inventory/Blueprint_and_Interfaces/BackPack_Master.PlayerSlots` (`self.EquipBackpack`)) Index)))))))

(fn `RetrievInventory`
  (returns (Inventory :type "Array of /Game/Sonik/Inventory/Structure/S_Slots Structure"))
  (return (`/Game/Sonik/Inventory/Blueprint_and_Interfaces/BackPack_Master.PlayerSlots` (`self.EquipBackpack`))))

(fn `UserConstructionScript`)