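; Master inventory Blueprint that stores items in a PlayerSlots array of data table row handles and amounts, using an "Empty" row name for free slots.
; AddItem merges into the first matching slot if its row allows stacking, otherwise fills the first empty slot.
; Removal works by item or index, rejecting amounts larger than the slot holds.
; Pickup and BeginPlay events are empty; the "Armor" socket equip logic is unconnected.
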(event `self.PickupInteraction`
  (params (Player :type "/Game/Sonik/New_Character/Character Object Reference")))

(event `self.ReceiveBeginPlay`)

(fn `AddItem`
  (params (Item :type "/Game/Sonik/Inventory/Structure/S_Slots Structure (by ref)"))
  (returns (Succes :type Boolean))
  (locals (LocalItem :type "/Game/Sonik/Inventory/Structure/S_Slots Structure"))
  (set `local.LocalItem` Item)
  (bind (_succes _index) (`self.FindStack` (`local.LocalItem`)))
  (if _succes
    (bind _success (`self.AddItemToSlot` (`local.LocalItem`) _index))
    (if _success
      (return _success)
      (else
        _)))
  (bind (_succes_2 _index_2) (`self.FindEmptySlot`))
  (if _succes_2
    (bind _success_2 (`self.AddItemToSlot` (`local.LocalItem`) _index_2))
    (return _success_2)
    (else
      (return false))))

(fn `AddItemToSlot`
  (params (item :type "/Game/Sonik/Inventory/Structure/S_Slots Structure") (Index :type Integer))
  (returns (Success :type Boolean))
  (locals (Localtem :type "/Game/Sonik/Inventory/Structure/S_Slots Structure") (localIndex :type Integer))
  (bind (_localtem_item _localtem_amount) (break `/Game/Sonik/Inventory/Structure/S_Slots` (`local.Localtem`)))
  (bind (_datatable _rowname) (break `DataTableRowHandle` _localtem_item))
  (bind (_output_item _output_amount) (break `/Game/Sonik/Inventory/Structure/S_Slots` (`|GetArrayItem` (`self.PlayerSlots`) (`local.localIndex`))))
  (bind (_datatable_2 _rowname_2) (break `DataTableRowHandle` _output_item))
  (set `local.Localtem` item)
  (set `local.localIndex` Index)
  (if (== _rowname_2 "Empty")
    (`KismetArrayLibrary.Array_Set` (`self.PlayerSlots`) (`local.localIndex`) (`local.Localtem`))
    (return true)
    (else
      (bind _returnvalue (`|GetDataTableRow` _datatable _rowname)
        (:`then`
          (if (and (`.CanStack_13_EE9C68654E665B3DD19AFEB7618792C9` (break `/Game/Sonik/Inventory/Structure/S_Inventory` _returnvalue)) (== _rowname_2 _rowname))
            (`KismetArrayLibrary.Array_Set` (`self.PlayerSlots`) (`local.localIndex`) (make `/Game/Sonik/Inventory/Structure/S_Slots` _localtem_item (+ _output_amount _localtem_amount)))
            (return true)
            (else
              (return false))))
        (:`RowNotFound`
          (return false))))))

(fn `FindEmptySlot`
  (returns (Succes :type Boolean) (Index :type Integer))
  (locals (LocalFound :type Boolean) (LocaalIndex :type Integer))
  (for (_array_element _array_index) (`self.PlayerSlots`)
    (if (== (`.RowName` (break `DataTableRowHandle` (`.Item_4_27233E2C43F0E942A1D6938F2A227CD8` (break `/Game/Sonik/Inventory/Structure/S_Slots` _array_element)))) "Empty")
      (set `local.LocalFound` true)
      (set `local.LocaalIndex` _array_index)
      (break)))
  (return (`local.LocalFound`) (`local.LocaalIndex`)))

(fn `FindStack`
  (params (Item :type "/Game/Sonik/Inventory/Structure/S_Slots Structure (by ref)"))
  (returns (Succes :type Boolean) (Index :type Integer) (Amount :type Integer))
  (locals (LocalFound :type Boolean) (LocalIndex :type Integer) (LocalAmount :type Integer))
  (for (_array_element _array_index) (`self.PlayerSlots`)
    (bind (_item _amount) (break `/Game/Sonik/Inventory/Structure/S_Slots` _array_element))
    (if (== (`.RowName` (break `DataTableRowHandle` _item)) (`.RowName` (break `DataTableRowHandle` (`.Item_4_27233E2C43F0E942A1D6938F2A227CD8` (break `/Game/Sonik/Inventory/Structure/S_Slots` Item)))))
      (set `local.LocalFound` true)
      (set `local.LocalIndex` _array_index)
      (set `local.LocalAmount` _amount)
      (break)))
  (return (`local.LocalFound`) (`local.LocalIndex`) (`local.LocalAmount`)))

(fn `RemoveAmountAtIndex`
  (params (Index :type Integer) (Amount :type Integer))
  (returns (Succes :type Boolean))
  (bind _playerslots (`self.PlayerSlots`))
  (bind (_output_item _output_amount) (break `/Game/Sonik/Inventory/Structure/S_Slots` (`|GetArrayItem` (`self.PlayerSlots`) Index)))
  (bind _returnvalue (- _output_amount Amount))
  (if (>= _returnvalue 0)
    (if (> _returnvalue 0)
      (`KismetArrayLibrary.Array_Set` _playerslots Index (make `/Game/Sonik/Inventory/Structure/S_Slots` _output_item _returnvalue))
      (else
        (`KismetArrayLibrary.Array_Set` _playerslots Index (make `/Game/Sonik/Inventory/Structure/S_Slots` (make `DataTableRowHandle` "/Game/Sonik/Inventory/Blueprint_and_Interfaces/ItemDataBase.ItemDataBase" "Empty")))))
    (return true)
    (else
      (return false))))

(fn `RemoveItem`
  (params (Item :type "/Game/Sonik/Inventory/Structure/S_Slots Structure (by ref)"))
  (returns (Success :type Boolean))
  (bind (_item _amount) (break `/Game/Sonik/Inventory/Structure/S_Slots` Item))
  (bind _playerslots (`self.PlayerSlots`))
  (bind (_succes _index _amount_2) (`self.FindStack` Item))
  (if _succes
    (bind _returnvalue (- _amount_2 _amount))
    (if (>= _returnvalue 0)
      (if (== _returnvalue 0)
        (`KismetArrayLibrary.Array_Set` _playerslots _index (make `/Game/Sonik/Inventory/Structure/S_Slots` (make `DataTableRowHandle` "/Game/Sonik/Inventory/Blueprint_and_Interfaces/ItemDataBase.ItemDataBase" "Empty")))
        (else
          (`KismetArrayLibrary.Array_Set` _playerslots _index (make `/Game/Sonik/Inventory/Structure/S_Slots` _item _returnvalue))))
      (return true)
      (else
        (return false)))
    (else
      (return false))))

(fn `UserConstructionScript`)