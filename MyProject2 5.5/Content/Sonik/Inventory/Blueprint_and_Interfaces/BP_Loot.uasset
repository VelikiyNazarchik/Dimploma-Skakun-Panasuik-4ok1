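; Lootable container actor that fills its inventory with random items and spills them into the world when a player interacts.
; The construction script rolls every ItemDataBase row against its Rarity, skipping zero and making higher values less likely.
; Interaction has the Player server-spawn each item at a small random offset, emptying the inventory.
; It also supports custom-depth outlines and a geometry-collection break before delayed destruction; inventory query functions are stubs.
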(event `/Game/Sonik/Inventory/Blueprint_and_Interfaces/AI_Interaction.StartInteraction`
  (params (Player :type "/Game/Sonik/New_Character/Character Object Reference"))
  (bind (_arrayindex _arrayelement) (`/Engine/EditorBlueprintResources/StandardMacros.ReverseForEachLoop` (`self.Inventory`))
    (:`LoopBody`
      (`/Game/Sonik/New_Character/Character.Server_SpawnItem` Player (+ (`self.K2_GetActorLocation`) (`KismetMathLibrary.MakeVector` (`KismetMathLibrary.RandomFloatInRange` 0.0 50.0) (`KismetMathLibrary.RandomFloatInRange` 0.0 50.0) 50.0)) _arrayelement)
      (`KismetArrayLibrary.Array_Remove` (`self.Inventory`) _arrayindex))))

(event `/Game/Sonik/Inventory/Blueprint_and_Interfaces/OutlineInterface.SelfDestroy`
  (bind _staticmeshcomponent (`self.StaticMeshComponent`))
  (`SceneComponent.SetVisibility` _staticmeshcomponent false false)
  (`PrimitiveComponent.SetCollisionResponseToAllChannels` _staticmeshcomponent "ECR_Ignore")
  (`AddComponent|NODE_AddGeometryCollectionComponent-0` :`bManualAttachment` true :`RelativeTransform` (`self.GetTransform`))
  (if true
    (`KismetSystemLibrary.Delay` 2.0)
    (`self.K2_DestroyActor`)))

(event `/Game/Sonik/Inventory/Blueprint_and_Interfaces/OutlineInterface.OutlineInteraction`
  (params (ON :type Boolean))
  (bind _staticmeshcomponent (`self.StaticMeshComponent`))
  (if ON
    (`PrimitiveComponent.SetRenderCustomDepth` _staticmeshcomponent true)
    (`PrimitiveComponent.SetCustomDepthStencilValue` _staticmeshcomponent 2)
    (else
      (`PrimitiveComponent.SetRenderCustomDepth` _staticmeshcomponent false)
      (`PrimitiveComponent.SetCustomDepthStencilValue` _staticmeshcomponent 0))))

(fn `HasSpace`
  (params (Item :type "/Game/Sonik/Inventory/Structure/S_Slots Structure"))
  (returns (Returne :type Boolean))
  (return false))

(fn `IsItemAvaible`
  (params (Item :type "/Game/Sonik/Inventory/Structure/S_Slots Structure") (Index :type Integer))
  (returns (Returne :type Boolean))
  (return false))

(fn `RetrievInventory`
  (returns (Inventory :type "Array of /Game/Sonik/Inventory/Structure/S_Slots Structure"))
  (return))

(fn `UserConstructionScript`
  (bind _outrownames (`DataTableFunctionLibrary.GetDataTableRowNames` "/Game/Sonik/Inventory/Blueprint_and_Interfaces/ItemDataBase.ItemDataBase"))
  (for _array_element _outrownames
    (bind _returnvalue (`|GetDataTableRow` "/Game/Sonik/Inventory/Blueprint_and_Interfaces/ItemDataBase.ItemDataBase" _array_element)
      (:`then`
        (bind (_name _desc _type _rarity) (break `/Game/Sonik/Inventory/Structure/S_Inventory` _returnvalue))
        (if (and (!= _rarity 0) (< _rarity (`KismetMathLibrary.RandomInteger` 100)))
          (`KismetArrayLibrary.Array_Add` (`self.Inventory`) (make `/Game/Sonik/Inventory/Structure/S_Slots` (make `DataTableRowHandle` "/Game/Sonik/Inventory/Blueprint_and_Interfaces/ItemDataBase.ItemDataBase" _array_element) 1)))))))